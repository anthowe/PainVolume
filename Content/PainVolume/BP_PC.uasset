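; BP_PC is the player controller that runs the death sequence and game restart for the player.
; OnDeath unpossesses the pawn, prints a debug message, starts a slow camera fade to blue that holds, and shows the WBP_Died widget.
; After a long delay it removes the widget and calls RestartGame on ThirdPersonGameMode.
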(event Custom|OnDeath
  (Pawn|UnPossess)
  (Development|PrintString "UNPOSSESS")
  (CameraFades|StartCameraFade (Game|GetPlayerCameraManager 0) 0.0 0.0 8.0 "(R=0.053107,G=0.161206,B=0.802083,A=1.000000)" false true)
  (bind _returnvalue (UserInterface|CreateWidget "/Game/PainVolume/WBP_Died.WBP_Died_C" self))
  (UserInterface|Viewport|AddtoViewport _returnvalue 0)
  (Utilities|FlowControl|Delay 3e+01)
  (Widget|RemovefromParent _returnvalue)
  (bind _asthird_person_game_mode (Utilities|Casting|CastToThirdPersonGameMode (Game|GetGameMode)))
  (Class|GameMode|RestartGame _asthird_person_game_mode))

(event EventBeginPlay)

(event EventTick
  (params (DeltaSeconds :type Float%20%28single-precision%29)))

(fn ConstructionScript)